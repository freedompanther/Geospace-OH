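; Test player character with basic first-person-style look, movement, jump, speed-only run and crouch, two-gun combat and a HUD created on BeginPlay.
; Number keys or mouse wheel set SwapGun, toggling rifle and pistol visibility and caching the gun actor via GetActorOfClass; rifle is the default.
; Reload and shoot calls forward to that actor.
; Shooting runs a self-repeating Delay loop passing fire state and camera transform, which continues after release.
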(event `InputAxis|Look Up/Down`
  (params (AxisValue :type "Float (single-precision)"))
  ;[1 1 1] Basic Look System (to be improved)
  (`self.AddControllerPitchInput` (* AxisValue 0.5)))

(event `InputAxis|Look Right/Left`
  (params (AxisValue :type "Float (single-precision)"))
  ;[1 1 1] Basic Look System (to be improved)
  (`self.AddControllerYawInput` (* AxisValue 0.5)))

(event `Key|Two`
  (params (Key :type "Key Structure"))
  ;[1 1 1] Swaping Weapons
  (:`Pressed`
    (set `self.SwapGun` 1)
    (if (== (`self.SwapGun`) 1) :!label _label
      (bind _returnvalue (`GameplayStatics.GetActorOfClass` "/Game/GunMechanics/Blueprints/BP_Pistol.BP_Pistol_C"))
      (set `self.Pistol Actor` _returnvalue)
      (`SceneComponent.SetVisibility` (`self.BP_Pistol`) true false)
      (`SceneComponent.SetVisibility` (`self.BP_Rifle`) false false)
      (else
        (bind _returnvalue_2 (`GameplayStatics.GetActorOfClass` "/Game/GunMechanics/Blueprints/BP_Rifle.BP_Rifle_C" :!label _label_2))
        (set `self.Rifle Actor` _returnvalue_2)
        (`SceneComponent.SetVisibility` (`self.BP_Rifle`) true false)
        (`SceneComponent.SetVisibility` (`self.BP_Pistol`) false false)))))

(event `InputAxis|Move Forward/Back`
  (params (AxisValue :type "Float (single-precision)"))
  ;[1 1 1] Basic Movement System (to be improved)
  (`self.AddMovementInput` (`self.GetActorForwardVector`) AxisValue))

(event `InputAction|Jumping`
  (params (Key :type "Key Structure"))
  ;[1 1 1] Basic Jump System (to be improved)
  (:`Pressed`
    (`self.Jump`))
  (:`Released`
    (`self.StopJumping`)))

(event `Key|One`
  (params (Key :type "Key Structure"))
  ;[1 1 1] Swaping Weapons
  (:`Pressed`
    (set `self.SwapGun` 0)
    (goto _label)))

(event `InputAxis|Move Right/Left`
  (params (AxisValue :type "Float (single-precision)"))
  ;[1 1 1] Basic Movement System (to be improved)
  (`self.AddMovementInput` (`self.GetActorRightVector`) AxisValue))

(event `Key|MouseScrollUp`
  (params (Key :type "Key Structure"))
  ;[1 1 1] Swaping Weapons
  (:`Pressed`
    (`/Engine/EditorBlueprintResources/StandardMacros.FlipFlop` :!label _label_3
      (:`A`
        (set `self.SwapGun` 1)
        (goto _label))
      (:`B`
        (set `self.SwapGun` 0)
        (goto _label)))))

(event `Key|MouseScrollDown`
  (params (Key :type "Key Structure"))
  ;[1 1 1] Swaping Weapons
  (:`Pressed`
    (goto _label_3)))

(event `InputAction|Reloading`
  (params (Key :type "Key Structure"))
  ;[1 1 1] Calls to Gun Actor to Reload
  (:`Pressed`
    (if (== (`self.SwapGun`) 1)
      (`/Game/GunMechanics/Blueprints/BP_Pistol.Reloading` (`self.Pistol Actor`))
      (else
        (`/Game/GunMechanics/Blueprints/BP_Rifle.Reloading` (`self.Rifle Actor`))))))

(event `self.ReceiveBeginPlay`
  (`|ExecutionSequence`
    (:`then_0`
      (goto _label_2))
    (:`then_1`
      (bind _returnvalue (`|CreateWidget` "/Game/UI/WB_GameHUD.WB_GameHUD_C"))
      (`UserWidget.AddToViewport` _returnvalue 0))))

(event `InputAction|Shooting`
  (params (Key :type "Key Structure"))
  (bind _isshooting_ (`self.IsShooting?`))
  (bind _camera (`self.Camera`))
  (bind _returnvalue (`SceneComponent.K2_GetComponentRotation` _camera))
  (bind _returnvalue_2 (`SceneComponent.K2_GetComponentLocation` _camera))
  ;[1 1 1] Calls to Gun Actor to Shoot
  (:`Pressed`
    (set `self.IsShooting?` true)
    (if (== (`self.SwapGun`) 1) :!label _label_4
      (`/Game/GunMechanics/Blueprints/BP_Pistol.Shooting` (`self.Pistol Actor`) _isshooting_ _returnvalue_2 _returnvalue)
      (else
        (`/Game/GunMechanics/Blueprints/BP_Rifle.Shooting` (`self.Rifle Actor`) _isshooting_ _returnvalue_2 _returnvalue)))
    (`KismetSystemLibrary.Delay` 0.01)
    (goto _label_4))
  (:`Released`
    (set `self.IsShooting?` false)
    (goto _label_4)))

(event `InputAction|Running`
  (params (Key :type "Key Structure"))
  (bind _charactermovement (`self.CharacterMovement`))
  (:`Pressed`
    (set `CharacterMovementComponent.MaxWalkSpeed` 20000.0 _charactermovement))
  (:`Released`
    (set `CharacterMovementComponent.MaxWalkSpeed` 600.0 _charactermovement)))

(event `InputAction|Crouching`
  (params (Key :type "Key Structure"))
  (bind _charactermovement (`self.CharacterMovement`))
  (:`Pressed`
    (set `CharacterMovementComponent.MaxWalkSpeed` 300.0 _charactermovement))
  (:`Released`
    (set `CharacterMovementComponent.MaxWalkSpeed` 600.0 _charactermovement)))

(fn `UserConstructionScript`)