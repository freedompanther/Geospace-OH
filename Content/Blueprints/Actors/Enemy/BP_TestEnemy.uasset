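; BP_TestEnemy is a test enemy actor that homes in on the player and awards points when killed.
; On BeginPlay it caches the player and starts two self-retriggering Delay loops in place of Tick.
; One interpolates location straight toward the player with random XY jitter, without sweep or navigation; the other rotates the actor to face them.
; Damage reduces Health, and at zero it adds Points to the player and destroys itself.
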(event `self.ReceiveBeginPlay`
  (bind _asbp_test_player (cast `/Game/Blueprints/Actors/Player/Blueprints/BP_TestPlayer` (`GameplayStatics.GetPlayerCharacter` 0)))
  (set `self.PlayerRef` _asbp_test_player)
  (`self.Ai Move To`)
  (`self.Ai Look At`))

(event `Ai Move To`
  (bind _returnvalue (`KismetMathLibrary.RandomFloatInRange` -100.0 100.0))
  (bind (_returnvalue_x _returnvalue_y _returnvalue_z) (`KismetMathLibrary.BreakVector` (`self.K2_GetActorLocation` (`self.PlayerRef`))))
  ;[1 1 1] Move Enemy to player in a strate line
  (`self.K2_SetActorLocation` (`KismetMathLibrary.VInterpTo_Constant` (`self.K2_GetActorLocation`) (`KismetMathLibrary.MakeVector` (+ _returnvalue_x _returnvalue) (+ _returnvalue_y _returnvalue) _returnvalue_z) (`GameplayStatics.GetWorldDeltaSeconds`) 1000.0))
  (`KismetSystemLibrary.Delay` 0.001)
  (`self.Ai Move To`))

(event `Ai Look At`
  ;[1 1 1] Make Enemy look at the player
  (`self.K2_SetActorRotation` (`KismetMathLibrary.FindLookAtRotation` (`SceneComponent.K2_GetComponentLocation` (`self.alien1`)) (`self.K2_GetActorLocation` (`self.PlayerRef`))))
  (`KismetSystemLibrary.Delay` 0.001)
  (`self.Ai Look At`))

(event `self.ReceiveAnyDamage`
  (params (Damage :type "Float (single-precision)") (DamageType :type "DamageType Object Reference") (InstigatedBy :type "Controller Object Reference") (DamageCauser :type "Actor Object Reference"))
  (bind _playerref (`self.PlayerRef`))
  (bind _output_get (set `self.Health` (`/Game/Blueprints/Actors/Enemy/BP_EnemyFunctions.DealDamage` (`self.Health`) Damage)))
  (if (<= _output_get 0.0)
    (set `/Game/Blueprints/Actors/Player/Blueprints/BP_TestPlayer.Points` (+ (`/Game/Blueprints/Actors/Player/Blueprints/BP_TestPlayer.Points` _playerref) (`self.Points`)) _playerref)
    (`self.K2_DestroyActor`)))

(fn `UserConstructionScript`)