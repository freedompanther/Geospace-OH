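; BP_EnemySpawner is an actor that spawns BP_TestEnemy actors around its own location until an allowed count is reached.
; On BeginPlay, SpawnEnemys places one enemy at a random X/Y offset from the scene root, stores it and increments SpawnedAmount.
; The event then calls itself after a short Delay, forming a staggered spawn loop that stops when SpawnedAmount equals AllowedSpawnAmount.
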(event `self.ReceiveBeginPlay`
  (`self.SpawnEnemys`))

(event `SpawnEnemys`
  (bind _returnvalue (`KismetMathLibrary.RandomFloatInRange` -1000.0 1000.0))
  (if (not (== (`self.SpawnedAmount`) (`self.AllowedSpawnAmount`)))
    (bind _returnvalue_2 (`|SpawnActorFromClass` "/Game/Blueprints/Actors/Enemy/BP_TestEnemy.BP_TestEnemy_C" (`KismetMathLibrary.MakeTransform` (+ (`SceneComponent.K2_GetComponentLocation` (`self.DefaultSceneRoot`)) (`KismetMathLibrary.MakeVector` _returnvalue _returnvalue))) "Undefined" "MultiplyWithRoot" null null))
    (set `self.SpawnReturnValue` _returnvalue_2)
    (bind _result (`/Engine/EditorBlueprintResources/StandardMacros.IncrementInt` (`self.SpawnedAmount`))
      (:`  `
        (set `self.SpawnedAmount` _result)
        (`KismetSystemLibrary.Delay` 0.1)
        (`self.SpawnEnemys`)))))

(fn `UserConstructionScript`)