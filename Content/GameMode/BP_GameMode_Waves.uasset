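; Wave game mode that starts the next enemy wave once no BP_TestEnemy actors remain.
; A delay-driven polling loop resets a ten-second countdown while enemies live, then counts down via StartNextRoundTimer, printing debug status.
; At zero, a DoOnce-guarded branch raises BP_EnemySpawner's allowed amount by five and triggers spawning.
; WaveSystem1 re-enters the loop without resetting the countdown; the guard resets when the spawn count reaches its limit.
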(event `self.ReceiveBeginPlay`
  (`self.Wave System`))

(event `Wave System`
  (bind _spawnerref (`self.SpawnerREF`))
  (bind _spawnerref_2 (`self.SpawnerREF`))
  (set `self.Time` 10)
  (`KismetSystemLibrary.Delay` 0.2 :!label _label)
  (bind _outactors (`GameplayStatics.GetAllActorsOfClass` "/Game/Blueprints/Actors/Enemy/BP_TestEnemy.BP_TestEnemy_C"))
  (bind _output_get (set `self.HowMenyEnemies` (`KismetArrayLibrary.Array_Length` _outactors)))
  (if (> _output_get 0)
    ;[1 1 1] Display the amount of enemys
    (`KismetSystemLibrary.PrintString` (`KismetStringLibrary.Conv_IntToString` (`self.HowMenyEnemies`)) true true (struct :`G` 0.66 :`B` 1.0 :`A` 1.0) 2.0 "1")
    (`KismetSystemLibrary.Delay` 0.001)
    (`self.Wave System`)
    (elif (== (`self.Time`) 0)
      ;[1 1 1] Spawn Enemys for next round
      (`/Engine/EditorBlueprintResources/StandardMacros.DoOnce` false :!label _label_2
        (:`Completed`
          (`KismetSystemLibrary.PrintString` "Starting Wave" true true (struct :`G` 0.66 :`B` 1.0 :`A` 1.0) 2.0 "3")
          (bind _returnvalue (`GameplayStatics.GetActorOfClass` "/Game/Blueprints/Actors/EnemySpawners/BP_EnemySpawner.BP_EnemySpawner_C"))
          (set `self.SpawnerREF` _returnvalue)
          (set `/Game/Blueprints/Actors/EnemySpawners/BP_EnemySpawner.AllowedSpawnAmount` (+ (`/Game/Blueprints/Actors/EnemySpawners/BP_EnemySpawner.AllowedSpawnAmount` (`self.SpawnerREF`)) 5) _spawnerref)
          (set `/Game/Blueprints/Actors/EnemySpawners/BP_EnemySpawner.SpawnedAmount` 0 _spawnerref)
          (`/Game/Blueprints/Actors/EnemySpawners/BP_EnemySpawner.SpawnEnemys` _spawnerref_2)
          (if (== (`/Game/Blueprints/Actors/EnemySpawners/BP_EnemySpawner.SpawnedAmount` _spawnerref_2) (`/Game/Blueprints/Actors/EnemySpawners/BP_EnemySpawner.AllowedSpawnAmount` _spawnerref_2)) :!label _label_3
            (`self.Wave System`)
            (goto _label_2 :!via `Reset`)
            (else
              (`KismetSystemLibrary.Delay` 0.001)
              (`self.WaveSystem1`)
              (goto _label_3)))))
      (else
        ;[1 1 1] Next Round Timer
        (`self.StartNextRoundTimer`)
        (`KismetSystemLibrary.PrintString` (`KismetStringLibrary.Concat_StrStr` "Next Rount Starting In" ":" (`KismetStringLibrary.Conv_IntToString` (`self.TimeTillNextRound`))) true true (struct :`G` 0.66 :`B` 1.0 :`A` 1.0) 2.0 "2")
        (`KismetSystemLibrary.Delay` 0.001)
        (`self.WaveSystem1`)))))

(event `WaveSystem1`
  (goto _label))

(event `StartNextRoundTimer`
  (`KismetSystemLibrary.Delay` 1.0)
  (bind _result (`/Engine/EditorBlueprintResources/StandardMacros.DecrementInt` (`self.Time`))
    (:`  `
      (set `self.TimeTillNextRound` (`KismetMathLibrary.Clamp` _result 0 10)))))

(fn `UserConstructionScript`)