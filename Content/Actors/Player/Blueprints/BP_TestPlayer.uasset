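; BP_TestPlayer is a test player character with basic movement, look, jump and run-speed controls.
; On BeginPlay it finds a BP_Gun in the level, with both SwapGun branches fetching the same class, and forwards shoot and reload input to it.
; Mouse wheel and number keys adjust the SwapGun index and mostly print it, but never reassign the gun after BeginPlay.
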(event `self.ReceiveBeginPlay`
  ;[1 1 1] Set Gun Actor to allow for inputs to be sent to the gun actor
  (if (== (`self.SwapGun`) 0)
    (bind _returnvalue (`GameplayStatics.GetActorOfClass` "/Game/GunMechanics/Blueprints/BP_Gun.BP_Gun_C"))
    (set `self.GunActor` _returnvalue)
    (else
      (bind _returnvalue_2 (`GameplayStatics.GetActorOfClass` "/Game/GunMechanics/Blueprints/BP_Gun.BP_Gun_C"))
      (set `self.GunActor` _returnvalue_2))))

(event `InputAxis|Move Forward/Back`
  (params (AxisValue :type "Float (single-precision)"))
  ;[1 1 1] Basic Movement System (to be improved)
  (`self.AddMovementInput` (`self.GetActorForwardVector`) AxisValue))

(event `InputAxis|Look Up/Down`
  (params (AxisValue :type "Float (single-precision)"))
  ;[1 1 1] Basic Look System (to be improved)
  (`self.AddControllerPitchInput` AxisValue))

(event `InputAction|Jumping`
  (params (Key :type "Key Structure"))
  ;[1 1 1] Basic Jump System (to be improved)
  (:`Pressed`
    (`self.Jump`))
  (:`Released`
    (`self.StopJumping`)))

(event `Key|MouseScrollUp`
  (params (Key :type "Key Structure"))
  ;[1 1 1] Swaping Weapons
  (:`Pressed`
    (if (>= (`self.SwapGun`) 0)
      (bind _result (`/Engine/EditorBlueprintResources/StandardMacros.DecrementInt` (`self.SwapGun`))
        (:`  `
          (set `self.SwapGun` _result)
          (`KismetSystemLibrary.PrintString` (`KismetStringLibrary.Conv_IntToString` (`self.SwapGun`)) :!label _label)))
      (else
        (set `self.SwapGun` 0)))))

(event `InputAxis|Look Right/Left`
  (params (AxisValue :type "Float (single-precision)"))
  ;[1 1 1] Basic Look System (to be improved)
  (`self.AddControllerYawInput` AxisValue))

(event `InputAxis|Move Right/Left`
  (params (AxisValue :type "Float (single-precision)"))
  ;[1 1 1] Basic Movement System (to be improved)
  (`self.AddMovementInput` (`self.GetActorRightVector`) AxisValue))

(event `Key|MouseScrollDown`
  (params (Key :type "Key Structure"))
  ;[1 1 1] Swaping Weapons
  (:`Pressed`
    (if (<= (`self.SwapGun`) 0)
      (bind _result (`/Engine/EditorBlueprintResources/StandardMacros.IncrementInt` (`self.SwapGun`))
        (:`  `
          (set `self.SwapGun` _result)
          (goto _label)))
      (else
        (set `self.SwapGun` 1)))))

(event `InputAction|Shooting`
  (params (Key :type "Key Structure"))
  ;[1 1 1] Calls to Gun Actor to Shoot
  (:`Pressed`
    (set `self.IsShooting?` true)
    (`/Game/GunMechanics/Blueprints/BP_Gun.Shooting` (`self.GunActor`) (`self.IsShooting?`) :!label _label_2))
  (:`Released`
    (set `self.IsShooting?` false)
    (goto _label_2)))

(event `InputAction|Reloading`
  (params (Key :type "Key Structure"))
  ;[1 1 1] Calls to Gun Actor to Reload
  (:`Pressed`
    (`/Game/GunMechanics/Blueprints/BP_Gun.Reloading` (`self.GunActor`))))

(event `Key|Two`
  (params (Key :type "Key Structure"))
  ;[1 1 1] Swaping Weapons
  (:`Pressed`
    (set `self.SwapGun` 1)
    (`KismetSystemLibrary.PrintString` (`KismetStringLibrary.Conv_IntToString` (`self.SwapGun`)) :!label _label_3)))

(event `Key|One`
  (params (Key :type "Key Structure"))
  ;[1 1 1] Swaping Weapons
  (:`Pressed`
    (set `self.SwapGun` 0)
    (goto _label_3)))

(event `InputAction|Running`
  (params (Key :type "Key Structure"))
  (bind _charactermovement (`self.CharacterMovement`))
  (:`Pressed`
    (set `CharacterMovementComponent.MaxWalkSpeed` 2000.0 _charactermovement))
  (:`Released`
    (set `CharacterMovementComponent.MaxWalkSpeed` 600.0 _charactermovement)))

(event `InputAction|Crouching`
  (params (Key :type "Key Structure")))

(fn `UserConstructionScript`)