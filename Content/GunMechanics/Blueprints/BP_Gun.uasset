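; BP_Gun is a firearm Blueprint that models a chambered round, a magazine and reserve ammo.
; Shooting repeats at FireRate while held, with ShootingFunction spawning a BP_Bullet at the muzzle, triggering sound and effects, then chambering the next round.
; Reloading refills the magazine from inventory and chambers a round if empty.
; CanShoot and CanReload checks gate both actions, and a looping debug print shows ammo counts.
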(event `self.ReceiveBeginPlay`
  ;[1 1 1] Debug UI
  (`KismetSystemLibrary.PrintString` (`KismetStringLibrary.Conv_IntToString` (`self.Chamber`)) :!label _label)
  (`KismetSystemLibrary.PrintString` (`KismetStringLibrary.Conv_IntToString` (`self.Mag`)))
  (`KismetSystemLibrary.PrintString` (`KismetStringLibrary.Conv_IntToString` (`self.Inventory`)))
  (`KismetSystemLibrary.Delay` 0.05)
  (goto _label))

(event `Shooting`
  (params (`IsShooting?` :type Boolean))
  ;[1 1 1] Shooting
  (set `self.Is Shooting?` `IsShooting?`)
  (bind _output_get (set `self.Can Shoot?` (`/Game/GunMechanics/Blueprints/BP_GunFunctions.CanShoot?` (`self.Chamber`) (`self.IsReloading?`) (`self.AlreadyShooting?`)) :!label _label_2))
  (if _output_get
    (set `self.AlreadyShooting?` true)
    (`self.ShootingFunction`)
    (`KismetSystemLibrary.Delay` (`self.FireRate`))
    (set `self.AlreadyShooting?` false)
    (if (`self.Is Shooting?`)
      (goto _label_2))
    (else
      (`GameplayStatics.PlaySound2D` null 1.0 1.0 0.0 null null)
      (`KismetSystemLibrary.PrintString` "Cant Shoot"))))

(event `Reloading`
  ;[1 1 1] Reloading
  (bind _output_get (set `self.IsReloading?` false))
  (if (`/Game/GunMechanics/Blueprints/BP_GunFunctions.CanReload?` _output_get (`self.AlreadyShooting?`) (`self.Mag`) (`self.MaxMag`) (`self.Inventory`))
    (set `self.IsReloading?` true)
    ;;[1 1 1] Reload Gun
    (bind (_magout _inventory_out) (`/Game/GunMechanics/Blueprints/BP_GunFunctions.Relaod` (`self.Inventory`) (`self.Mag`) (`self.MaxMag`)))
    (set `self.Mag` _magout)
    (set `self.Inventory` _inventory_out)
    ;;[1 1 1] Check if a round is in the chamber
    (if (== (`self.Chamber`) 0)
      ;;[1 1 1] Check if mag has ammo
      (if (> (`self.Mag`) 0)
        ;;[1 1 1] Take round from mag into chamber if there isnt already one when reloading
        (bind _result (`/Engine/EditorBlueprintResources/StandardMacros.DecrementInt` (`self.Mag`))
          (:`  `
            (set `self.Mag` _result)
            (set `self.Chamber` 1)
            (set `self.IsReloading?` false)))
        (else
          (`KismetSystemLibrary.PrintString` "Out Of Ammo")
          (set `self.IsReloading?` false)))
      (else
        (`KismetSystemLibrary.PrintString` "Bullet In chamber")
        (set `self.IsReloading?` false)))
    (else
      (`KismetSystemLibrary.PrintString` "Can't Reload"))))

(fn `ShootingFunction`
  (`|ExecutionSequence`
    (:`then_0`
      (set `self.Chamber` 0))
    (:`then_1`
      (`self.Spawn Bullet`))
    (:`then_2`
      (`GameplayStatics.CreateSound2D` null 1.0 1.0 0.0 null))
    (:`then_3`
      (`NiagaraFunctionLibrary.SpawnSystemAtLocation` null))
    (:`then_4`
      (if (not (== (`self.Mag`) 0))
        (bind _result (`/Engine/EditorBlueprintResources/StandardMacros.DecrementInt` (`self.Mag`))
          (:`  `
            (set `self.Mag` _result)
            (set `self.Chamber` 1)
            (return)))
        (else
          (`KismetSystemLibrary.PrintText` "Reload")
          (set `self.MustReload?` true)
          (return))))))

(fn `Spawn Bullet`
  (`|SpawnActorFromClass` "/Game/GunMechanics/Blueprints/BP_Bullet.BP_Bullet_C" (`SceneComponent.K2_GetComponentToWorld` (`self.MuzzleLocation`)) "Undefined" "MultiplyWithRoot" null null))

(fn `UserConstructionScript`)