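; BP_ProjectileFunctions provides helper functions for simulating bullets as stepped line traces with simple ballistics.
; Each step projects an end position from velocity and delta time, then a debug-drawn Visibility trace reports hits, leaving its ActorsToIgnore input unused.
; Gravity, scaled by bullet mass, updates vertical velocity, with a variant adding drag to Z only.
; The Drag formula is computed but not wired to an output.
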(fn `Apply Gravity`
  (params (`Velocity In` :type "Vector Structure") (Gravity :type "Float (double-precision)") (`Bullet Mass` :type "Float (double-precision)") (`Delta Time` :type "Float (double-precision)"))
  (returns (`Vector Out` :type "Vector Structure"))
  ;[1 1 1] Conputing Gravity
  (return (+ `Velocity In` (* (`KismetMathLibrary.MakeVector` 0.0 0.0 (* (* Gravity 100.0) `Bullet Mass` -1.0)) `Delta Time`))))

(fn `Apply Gravity and Drag`
  (params (`Velocity In` :type "Vector Structure") (Gravity :type "Float (double-precision)") (`Bullet Mass` :type "Float (double-precision)") (`Delta Time` :type "Float (double-precision)") (`Air Density` :type "Float (double-precision)") (`Bullet Speed` :type "Float (double-precision)") (`Cross Section` :type "Float (double-precision)") (`Drag Coefficincy` :type "Float (double-precision)"))
  (returns (`Vector Out` :type "Vector Structure"))
  (return (+ `Velocity In` (* (`KismetMathLibrary.MakeVector` 0.0 0.0 (+ (* (* Gravity 100.0) `Bullet Mass` -1.0) (* (/ (* (* (* `Air Density` (`KismetMathLibrary.Square` `Bullet Speed`)) `Cross Section`) `Drag Coefficincy`) 2.0) -1.0))) `Delta Time`))))

(fn `Find Start and End Position`
  (params (`Start In` :type "Vector Structure") (Velocity :type "Vector Structure") (`Delta Time` :type "Float (double-precision)"))
  (returns (`Sart Position` :type "Vector Structure") (`End Position` :type "Vector Structure"))
  ;[1 1 1] Find End Position and allow Start Position toi Pass through
  (return `Start In` (+ `Start In` (* Velocity `Delta Time`))))

(fn `Spawn Line Trace`
  (params (Start :type "Vector Structure") (End :type "Vector Structure") (ActorsToIgnore :type "Array of Actor Object Reference (by ref)"))
  (returns (OutHit :type "HitResult Structure") (`Did Hit?` :type Boolean))
  ;[1 1 1] Creates a line Trace
  (bind (_outhit _returnvalue) (`KismetSystemLibrary.LineTraceSingle` :`Start` Start :`End` End :`TraceChannel` "TraceTypeQuery1" :`DrawDebugType` "ForDuration"))
  (return _outhit _returnvalue))