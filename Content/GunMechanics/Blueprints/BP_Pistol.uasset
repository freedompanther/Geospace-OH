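; BP_Pistol is a pistol weapon actor that fires BP_9mm rounds, tracks chamber, magazine and inventory ammo, and can rotate toward a look-at point.
; Shooting checks CanShoot, then spawns the bullet from the camera transform with sound and muzzle flash, chambers the next round and waits out the fire rate.
; Reloading refills the magazine from inventory and chambers a round if empty.
; An ammo debug print loop is left unconnected.
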(event `WeaponLookAt`
  (params (LookAtLocation :type "Vector Structure"))
  (`self.K2_SetActorRotation` (`KismetMathLibrary.FindLookAtRotation` (`self.K2_GetActorLocation`) LookAtLocation)))

(event `self.ReceiveBeginPlay`
  ;[1 1 1] Debug UI
)

(event `Shooting`
  (params (`IsShooting?` :type Boolean) (CameraLocation :type "Vector Structure") (CameraRotation :type "Rotator Structure"))
  ;[1 1 1] Shooting
  (if `IsShooting?`
    (set `self.Camera Location` CameraLocation)
    (set `self.Camera Rotation` CameraRotation)
    (bind _output_get (set `self.Can Shoot?` (`/Game/GunMechanics/Blueprints/BP_GunFunctions.CanShoot?` (`self.Chamber`) (`self.IsReloading?`) (`self.AlreadyShooting?`))))
    (if _output_get
      (set `self.AlreadyShooting?` true)
      (`self.ShootingFunction`)
      (`KismetSystemLibrary.Delay` (`self.FireRate`))
      (set `self.AlreadyShooting?` false)
      (else
        (`GameplayStatics.PlaySound2D` null 1.0 1.0 0.0 null null)
        (`KismetSystemLibrary.PrintString` "Cant Shoot")))))

(event `Reloading`
  ;[1 1 1] Reloading
  (bind _output_get (set `self.IsReloading?` false))
  (if (`/Game/GunMechanics/Blueprints/BP_GunFunctions.CanReload?` _output_get (`self.AlreadyShooting?`) (`self.Mag`) (`self.MaxMag`) (`self.Inventory`))
    (set `self.IsReloading?` true)
    ;;[1 1 1] Reload Gun
    (bind (_inventory_out _magout) (`/Game/GunMechanics/Blueprints/BP_GunFunctions.Relaod` (`self.Inventory`) (`self.Mag`) (`self.MaxMag`)))
    (set `self.Inventory` _inventory_out)
    (set `self.Mag` _magout)
    ;;[1 1 1] Check if a round is in the chamber
    (if (== (`self.Chamber`) 0)
      ;;[1 1 1] Check if mag has ammo
      (if (> (`self.Mag`) 0)
        ;;[1 1 1] Take round from mag into chamber if there isnt already one when reloading
        (bind _result (`/Engine/EditorBlueprintResources/StandardMacros.DecrementInt` (`self.Mag`))
          (:`  `
            (set `self.Mag` _result)
            (set `self.Chamber` 1)
            (`KismetSystemLibrary.Delay` 0.3)
            (set `self.IsReloading?` false)))
        (else
          ;;[1 1 1] Finish reloading without without puting a round in the chamber as there is already one in.
          (`KismetSystemLibrary.Delay` 0.2 :!label _label)
          (set `self.IsReloading?` false)))
      (else
        (goto _label)))
    (else
      (`KismetSystemLibrary.PrintString` "Can't Reload"))))

(fn `ShootingFunction`
  (bind _muzzlelocation (`self.MuzzleLocation`))
  (`|ExecutionSequence`
    (:`then_0`
      (set `self.Chamber` 0))
    (:`then_1`
      (`self.Spawn Bullet`))
    (:`then_2`
      (`GameplayStatics.CreateSound2D` null 1.0 1.0 0.0 null))
    (:`then_3`
      (`NiagaraFunctionLibrary.SpawnSystemAtLocation` "/Game/VFX/MuzzleFlash/MuzzleFlashTest.MuzzleFlashTest" (`SceneComponent.RelativeLocation` _muzzlelocation) (`SceneComponent.RelativeRotation` _muzzlelocation) (10.0 10.0 10.0)))
    (:`then_4`
      (if (not (== (`self.Mag`) 0))
        (bind _result (`/Engine/EditorBlueprintResources/StandardMacros.DecrementInt` (`self.Mag`))
          (:`  `
            (set `self.Mag` _result)
            (set `self.Chamber` 1)
            (return)))
        (else
          (`KismetSystemLibrary.PrintText` "Reload")
          (set `self.MustReload?` true)
          (return))))))

(fn `Spawn Bullet`
  (`|SpawnActorFromClass` "/Game/GunMechanics/Blueprints/BP_9mm.BP_9mm_C" (`KismetMathLibrary.MakeTransform` (`self.Camera Location`) (`self.Camera Rotation`)) "Undefined" "MultiplyWithRoot" null null))

(fn `UserConstructionScript`)