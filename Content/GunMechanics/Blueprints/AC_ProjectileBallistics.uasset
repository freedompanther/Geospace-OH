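; Actor component that drives its owning projectile as a simulated bullet with gravity-affected travel, hit damage and a limited lifespan.
; On BeginPlay it sets velocity from the owner's forward vector, then runs a Delay-based fixed-timestep loop, provided the player casts to BP_TestPlayer.
; Each step line-traces the next segment, then either applies fixed damage and destroys the owner, or teleportlessly moves it and updates velocity for gravity and mass.
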(event `self.ReceiveBeginPlay`
  (bind _owner (`self.Owner`))
  (bind (_sart_position _end_position) (`/Game/GunMechanics/Blueprints/BP_ProjectileFunctions.Find Start and End Position` (`Actor.K2_GetActorLocation` _owner) (`self.Velocity`) (`self.FixedDeltaTime`)))
  ;[1 1 1] On Begin Play get Actor this Actor Component is place in
  (set `self.Owner` (`self.GetOwner`))
  ;[1 1 1] Get Player Ref
  (bind _asbp_test_player (cast `/Game/Actors/Player/Blueprints/BP_TestPlayer` (`GameplayStatics.GetPlayerCharacter` 0)))
  (set `self.Player Ref` _asbp_test_player)
  (`|ExecutionSequence`
    (:`then_0`
      ;[1 1 1] Functions done once on begin play
      (set `self.Velocity` (* (`Actor.GetActorForwardVector` _owner) (`self.BulletSpeed`)))
      (`KismetArrayLibrary.Array_Add` (`self.Ignore Actor`) (`self.Owner`))
      (`KismetSystemLibrary.Delay` (`self.LifeSpan`))
      (`Actor.K2_DestroyActor` (`self.Owner`)))
    (:`then_1`
      ;[1 1 1] Looped Functions
      (set `self.Sart Position` _sart_position :!label _label)
      (set `self.End Position` _end_position)
      (bind (_outhit _did_hit_) (`/Game/GunMechanics/Blueprints/BP_ProjectileFunctions.Spawn Line Trace` (`self.Sart Position`) (`self.End Position`) (`self.Ignore Actor`)))
      (if _did_hit_
        (bind _output_get (set `self.Out Hit` _outhit))
        (`/Game/GunMechanics/Blueprints/BP_GunFunctions.Apply Damage` _output_get 15.0 (`self.Owner`))
        (`Actor.K2_DestroyActor` (`self.Owner`))
        (else
          (`Actor.K2_SetActorLocation` (`self.Owner`) (`self.End Position`) false false)
          (set `self.Velocity` (`/Game/GunMechanics/Blueprints/BP_ProjectileFunctions.Apply Gravity` (`self.Velocity`) (`self.Gravity`) (`self.BulletMass`) (`self.FixedDeltaTime`)))
          (`KismetSystemLibrary.Delay` (`self.FixedDeltaTime`))
          (goto _label))))))